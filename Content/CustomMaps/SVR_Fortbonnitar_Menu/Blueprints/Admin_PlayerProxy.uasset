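; Per-player proxy for an admin menu in a Pavlov custom map, exposing kick, delayed teleport, walk speed toggle, kill and Admin "ghost" skin actions.
; On BeginPlay the authority asks PlayerInfo to spawn the menu; the proxy's own hand-attached menu and selector code is unwired.
; Name loaders build player lists through GameLogic_Admin, and RepNotifies apply player tags such as Murderer.
; Several events and RepNotifies are empty stubs.
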(event Custom|Make%20Ghost
  (Class|PavlovPlayerProxy|SetPlayerSkin "Admin"))

(event Custom|Kill%20Player
  (params (Remove%20Body :type Boolean))
  (Variables|Gameplay|SetRemove%20Body Remove%20Body)
  (Game|Damage|ApplyDamage (Class|PavlovPlayerProxy|GetPawn) 3e+03 0 0))

(event Custom|Death%20Override)

(event Custom|Load%20All%20Names
  (Variables|Gameplay|SetAll%20Names (Utilities|Array|MakeArray))
  (Utilities|Casting|CastToGameLogic_Admin (Class|PavlovLibrary|GetGameLogic))
  (for _array_element (Variables|Core|GetAlive%20Players)
    (Utilities|Array|Add (Variables|Gameplay|GetAll%20Names) (Utilities|GetDisplayName _array_element))))

(event Custom|Teleport%20Player
  (params (Location%20Array :type Array%20of%20Box%20Component%20Object%20References) (Index :type Integer) (Delay :type Float%20%28single-precision%29))
  (if (== Delay 0.0)
    _
    (else
      (Utilities|FlowControl|Delay Delay)))
  (Transformation|SetActorTransform (Class|PavlovPlayerProxy|GetPawn) (Transformation|GetWorldTransform (Utilities|Array|Get(acopy) Location%20Array Index))))

(event Custom|Server%20Teleport%20Player
  (params (Location%20Array :type Array%20of%20Box%20Component%20Object%20References) (Index :type Integer) (Delay :type Float%20%28single-precision%29))
  (CallFunction|TeleportPlayer Location%20Array Index Delay))

(event Custom|Set%20Walk%20Speed
  (params (Slow :type Boolean))
  (bind _ascharacter (Utilities|Casting|CastToCharacter (Class|PavlovPlayerProxy|GetPawn)))
  (Variables|/Script/Engine.CharacterMovementComponent|SetMaxWalkSpeed (Variables|/Script/Engine.Character|GetCharacterMovement _ascharacter) (Math|Float|SelectFloat 6e+02 1.2e+03 Slow)))

(event Custom|Server%20Kick
  (CallFunction|ClientKick))

(event Custom|Client%20Kick
  (Development|ExecuteConsoleCommand "disconnect" 0))

(event Custom|Server%20Mark%20Dominant
  (bind _returnvalue (Class|PavlovPlayerProxy|GetPawn))
  (bind _right_hand (CallFunction|GetHands _returnvalue))
  (bind _asadmin_player_info (Utilities|Casting|CastToAdmin_PlayerInfo (Class|PavlovLibrary|GetPlayerInfo (Variables|/Script/Engine.Pawn|GetPlayerState _returnvalue))))
  (Default|MarkDominant _asadmin_player_info (== _right_hand (Transformation|GetAttachParent (Transformation|GetAttachParent (Transformation|GetAttachParent (.dominanthand (Variables|Default|GetHandsProxy)))))))
  (Variables|Default|SetPlayer%20Info _asadmin_player_info))

(event Custom|Load%20Names
  (Variables|Core|SetAlive%20Players (Utilities|Array|MakeArray))
  (Variables|Gameplay|SetName%20Array (Utilities|Array|MakeArray))
  (Utilities|Casting|CastToGameLogic_Admin (Class|PavlovLibrary|GetGameLogic))
  (for _array_element (Variables|Core|GetAlive%20Players)
    (bind _playerstatus (Class|PavlovProxyStatics|GetPavlovPlayerStatus _array_element))
    (if (not (.bdead _playerstatus))
      (Utilities|Array|AddUnique (Variables|Core|GetAlive%20Players) (.playerstate _playerstatus))
      (Utilities|Array|AddUnique (Variables|Gameplay|GetName%20Array) (Variables|/Script/Engine.PlayerState|GetPlayerName (.playerstate _playerstatus))))))

(event EventOnPlayerDeath
  (params (KilledActor :type Actor%20Object%20Reference)))

(event EventBeginPlay
  (Networking|SwitchHasAuthority
    (:Authority
      (Default|ServerSpawnMenu (Variables|Default|GetPlayer%20Info)))))

(event EventTick
  (params (DeltaSeconds :type Float%20%28single-precision%29)))

(fn ConstructionScript)

(fn OnRepCode)

(fn OnRepSetTags
  (CallFunction|ManageTags (Variables|/Script/Engine.Pawn|GetPlayerState (Class|PavlovPlayerProxy|GetPawn)) true "Murderer"))

(fn OnRepTotalTasks)

(fn OnRepComsScrampledEg
  (if (Variables|Gameplay|GetComs%20Scrampled%20Eg)
    (Actor|Tick|SetActorTickEnabled true)))

(fn GetRoundState
  (bind _asgame_logic_admin (Utilities|Casting|CastToGameLogic_Admin (Class|PavlovLibrary|GetGameLogic)))
  (return (Utilities|Enum|NotEqual(Enum) (Class|PavlovGameLogic|GetRoundState _asgame_logic_admin) "Started")))

(fn OnRepSetJesterTag)

(fn OnRepSetTag
  (CallFunction|ManageTags (Variables|/Script/Engine.Pawn|GetPlayerState (Class|PavlovPlayerProxy|GetPawn)) true (Variables|Default|GetSet%20Tag)))

(fn OnRepMurderer
  (CallFunction|ManageTags (Variables|/Script/Engine.Pawn|GetPlayerState (Class|PavlovPlayerProxy|GetPawn)) true "Murderer"))