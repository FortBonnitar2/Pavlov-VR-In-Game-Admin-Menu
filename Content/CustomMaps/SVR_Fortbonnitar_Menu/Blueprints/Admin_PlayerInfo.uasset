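; Per-player info Blueprint for a Pavlov VR admin mod, providing a moderator-only in-world menu and player moderation actions.
; ServerSpawnMenu checks the display name against the moderator list, then ClientMenu attaches the menu and selector to the off and main motion-controller hands.
; Name-based actions kick players through a client disconnect command or apply Ghost, Clown and Naked skins.
; It also ends matches, refreshes the widget's name list and handles radio channel, static sound and quality.
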(event Custom|Set%20Channel
  (params (Index :type Integer))
  (Class|PavlovPlayerInfo|SetRadioChannel Index))

(event Custom|Set%20Quality%20Level
  (params (Quality :type Byte))
  (Variables|Default|SetQuality Quality))

(event Custom|Kick%20Player
  (params (Name :type String))
  (bind _asgame_state (Utilities|Casting|CastToGameState (Game|GetGameState)))
  (for _array_element (Variables|/Script/Engine.GameStateBase|GetPlayerArray _asgame_state)
    (if (Utilities|Enum|Equal(Enum) (Utilities|GetDisplayName _array_element) Name)
      (bind _asadmin_player_info (Utilities|Casting|CastToAdmin_PlayerInfo (Class|PavlovLibrary|GetPlayerInfo)))
      (CallFunction|ServerKick _asadmin_player_info))))

(event Custom|Server%20Kick
  (CallFunction|ClientKick))

(event Custom|Client%20Kick
  (Development|ExecuteConsoleCommand "disconnect" 0))

(event Custom|Play%20Static%20Loop
  (Utilities|IsValid (Variables|Default|GetStatic)
    (:Is%20Not%20Valid
      (bind _returnvalue (Audio|SpawnSound2D 0 1.0 1.0 0.0 0))
      (bind _output_get (Variables|Default|SetStatic _returnvalue))
      (Utilities|FlowControl|Delay 3e+01)
      (Audio|Components|Audio|Stop _output_get))))

(event Custom|Make%20Clown
  (params (Name :type String))
  (Utilities|Casting|CastToGameLogic_Admin (Class|PavlovLibrary|GetGameLogic))
  (for _array_element (Variables|Default|GetPlayers)
    (if (Utilities|Enum|Equal(Enum) (Utilities|GetDisplayName _array_element) Name)
      (Utilities|Casting|CastToAdmin_PlayerInfo (Class|PavlovLibrary|GetPlayerInfo))
      (bind _asadmin_player_proxy (Utilities|Casting|CastToAdmin_PlayerProxy (Class|PavlovLibrary|GetPlayerProxy)))
      (Class|PavlovPlayerProxy|SetPlayerSkin _asadmin_player_proxy "Clown"))))

(event Custom|Load%20All%20Names
  (Variables|Default|SetAll%20Names (Utilities|Array|MakeArray))
  (bind _asgame_state (Utilities|Casting|CastToGameState (Game|GetGameState)))
  (for _array_element (Variables|/Script/Engine.GameStateBase|GetPlayerArray _asgame_state)
    (Utilities|Array|Add (Variables|Default|GetAll%20Names) (Utilities|GetDisplayName _array_element)))
  (CallFunction|ClientLoadNames))

(event Custom|Client%20Load%20Names
  (bind _asadmin_widget (Utilities|Casting|CastToAdmin_Widget (UserInterface|GetUserWidgetObject (Variables|/Game/CustomMaps/SVR_Fortbonnitar_Menu/Widget/AdminMenu/AdminMenu.AdminMenu_C|GetWidget (Variables|Default|GetWorld%20Menu)))))
  (Default|LoadedNames _asadmin_widget))

(event Custom|Server%20Spawn%20Menu
  (bind _player_valid (CallFunction|MenuCheck))
  (if _player_valid
    (CallFunction|ClientMenu)))

(event Custom|Client%20Menu
  (bind _returnvalue (Game|Player|GetPlayerPawn 0))
  (bind (_mainhand _offhand) (CallFunction|GetHands _returnvalue (Variables|Default|GetRight%20Hand%20Dominant)))
  (bind _returnvalue_2 (Game|SpawnActorfromClass "/Game/CustomMaps/SVR_Fortbonnitar_Menu/Widget/AdminMenu/Selector.Selector_C" (Transformation|GetWorldTransform _mainhand) "Undefined" _returnvalue 0))
  (bind _output_get (Variables|Default|SetWidget%20Ineractor _returnvalue_2))
  (Transformation|AttachComponentToComponent _output_get _mainhand "None" "SnapToTarget" "SnapToTarget" "KeepWorld" true)
  (bind _returnvalue_3 (Game|SpawnActorfromClass "/Game/CustomMaps/SVR_Fortbonnitar_Menu/Widget/AdminMenu/AdminMenu.AdminMenu_C" (Transformation|GetWorldTransform _offhand) "Undefined" _returnvalue 0))
  (bind _output_get_2 (Variables|Default|SetWorld%20Menu _returnvalue_3))
  (Transformation|AttachComponentToComponent _output_get_2 _offhand "None" "SnapToTarget" "SnapToTarget" "KeepWorld" true))

(event Custom|Mark%20Dominant
  (params (Right%20Hand%20Dominant :type Boolean))
  (Variables|Default|SetRight%20Hand%20Dominant Right%20Hand%20Dominant))

(event Custom|End%20Match
  (bind _asgame_logic_admin (Utilities|Casting|CastToGameLogic_Admin (Class|PavlovLibrary|GetGameLogic)))
  (Class|PavlovGameLogic|SetRoundState _asgame_logic_admin "Ended"))

(event Custom|Make%20Naked
  (params (Name :type String))
  (Utilities|Casting|CastToGameLogic_Admin (Class|PavlovLibrary|GetGameLogic))
  (for _array_element (Variables|Default|GetPlayers)
    (if (Utilities|Enum|Equal(Enum) (Utilities|GetDisplayName _array_element) Name)
      (Utilities|Casting|CastToAdmin_PlayerInfo (Class|PavlovLibrary|GetPlayerInfo))
      (bind _asadmin_player_proxy (Utilities|Casting|CastToAdmin_PlayerProxy (Class|PavlovLibrary|GetPlayerProxy)))
      (Class|PavlovPlayerProxy|SetPlayerSkin _asadmin_player_proxy "Naked"))))

(event Custom|Make%20Ghost
  (params (Name :type String))
  (Utilities|Casting|CastToGameLogic_Admin (Class|PavlovLibrary|GetGameLogic))
  (for _array_element (Variables|Default|GetPlayers)
    (if (Utilities|Enum|Equal(Enum) (Utilities|GetDisplayName _array_element) Name)
      (Utilities|Casting|CastToAdmin_PlayerInfo (Class|PavlovLibrary|GetPlayerInfo))
      (bind _asadmin_player_proxy (Utilities|Casting|CastToAdmin_PlayerProxy (Class|PavlovLibrary|GetPlayerProxy)))
      (Class|PavlovPlayerProxy|SetPlayerSkin _asadmin_player_proxy "Ghost"))))

(fn GetHands
  (params (Pawn :type Pawn%20Object%20Reference) (Right%20Hand%20Dominant :type Boolean))
  (for _array_element (Components|GetChildrenComponents (Variables|/Script/Engine.Actor|GetRootComponent Pawn) true)
    (bind _asmotion_controller_component (Utilities|Casting|CastToMotionControllerComponent _array_element))
    (switch name (Variables|/Script/HeadMountedDisplay.MotionControllerComponent|GetMotionSource _asmotion_controller_component)
      (:Left
        (LocalVariables|SetLeft%20Hand _asmotion_controller_component))
      (:Right
        (LocalVariables|SetRight%20Hand _asmotion_controller_component)))))

(fn MenuCheck
  (bind (_playerstatus _bsucceeded) (Class|PavlovProxyStatics|GetPavlovPlayerStatus (Class|PavlovPlayerInfo|GetPlayerState)))
  (if _bsucceeded
    (Utilities|Casting|CastToGameLogic_Admin (Class|PavlovLibrary|GetGameLogic))
    (bind (_bsuccessful _mods) (Class|PavlovLibrary|GetModerators))
    (return (and _bsuccessful (Utilities|Array|ContainsItem _mods (Utilities|GetDisplayName (.Pawn (Utilities|Struct|BreakPavlovPlayerStatus _playerstatus))))))))